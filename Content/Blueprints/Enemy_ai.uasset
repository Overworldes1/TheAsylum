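; Enemy pawn that hunts the player by sound, using live audio input from an AudioCapture component.
; When the audio envelope crosses a loudness threshold, it runs AIMoveTo toward the player's current location.
; From BeginPlay, it also loops a white-noise sound at its own location, with a random delay of a few seconds between plays.
; A random-wander patrol loop exists but is disconnected, so it never runs.
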(event OnAudioEnvelopeValue(AudioCapture)
  (params (EnvelopeValue :type Float%20%28single-precision%29))
  ;[1 1 1] Enemy Audio movement
  (if (>= EnvelopeValue 0.2)
    (AI|AIMoveTo self (Transformation|GetActorLocation (Game|Player|GetPlayerPawn 0)) 0 5.0 false)))

(event EventBeginPlay
  (Utilities|FlowControl|Sequence
    (:then_1
      (Audio|PlaySoundatLocation "/Engine/EngineSounds/WhiteNoise.WhiteNoise" (Transformation|GetActorLocation) "0, 0, 0" 1.0 1.0 0.0 0 0 0 0 :!label _label)
      (Utilities|FlowControl|Delay (Math|Conversions|ToFloat(Integer) (Math|Random|RandomIntegerinRange 3 7)))
      (goto _label))))

(fn ConstructionScript)