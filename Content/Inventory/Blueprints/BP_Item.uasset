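; BP_Item is an inventory item actor placed in the world, with a text label that appears when the player is near.
; The construction script applies the mesh from its Item data and disables physics simulation.
; BeginPlay zeroes the label's world rotation, and Tick toggles its visibility by polling the distance to the first player's character against a fixed radius.
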(event EventBeginPlay
  (Transformation|SetWorldRotation (Variables|Default|GetTextRender) "0, 0, 0" false false))

(event Collision|EventActorBeginOverlap
  (params (OtherActor :type Actor%20Object%20Reference)))

(event EventTick
  (params (DeltaSeconds :type Float%20%28single-precision%29))
  (if (>= (Math|Vector|VectorLength (- (Transformation|GetActorLocation (Game|GetPlayerCharacter 0)) (Transformation|GetActorLocation))) 2e+02)
    (Rendering|SetVisibility (Variables|Default|GetTextRender) false false)
    (else
      (Rendering|SetVisibility (Variables|Default|GetTextRender) true false))))

(fn ConstructionScript
  (bind _staticmesh (Variables|Default|GetStaticMesh))
  (Components|StaticMesh|SetStaticMesh _staticmesh (.Mesh (Utilities|Struct|BreakS_Item_Structure (Variables|Default|GetItem))))
  (Physics|SetSimulatePhysics _staticmesh false))